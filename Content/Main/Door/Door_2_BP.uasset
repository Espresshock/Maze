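; Puzzle door that opens once both its blue and orange trigger volumes have registered their matching trigger actors.
; Each volume's begin overlap sets its flag by exact class check and clears it for any other actor; when both are true, IsOpen is set and audio plays.
; While open, Tick, set to a 0.01s interval, uses FInterpTo to ease the slab's relative Z toward TargetLocation.
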(event `self.ReceiveBeginPlay`
  (`self.SetActorTickInterval` 0.01))

(event `self.ReceiveTick`
  (params (DeltaSeconds :type "Float (single-precision)"))
  (bind _slabdoor_cube (`self.slabdoor_Cube`))
  (bind _target_location (`self.Target Location`))
  (bind _z (.z (.location (`SceneComponent.GetRelativeTransform` _slabdoor_cube))))
  (if (`self.IsOpen`)
    (`SceneComponent.K2_SetRelativeTransform` _slabdoor_cube (`KismetMathLibrary.MakeTransform` (`KismetMathLibrary.MakeVector` 0.0 0.0 (`KismetMathLibrary.FInterpTo` _z _target_location (`self.GetActorTickInterval`) 0.2))) false false)
    (if (not (== _z _target_location))
      (set `self.IsOpen` true))))

(event `self.TriggerVolBlue.OnActorBeginOverlap`
  (params (OverlappedActor :type "Actor Object Reference") (OtherActor :type "Actor Object Reference"))
  (bind _audio (`self.Audio`))
  (if (== (`GameplayStatics.GetObjectClass` OtherActor) "/Game/Main/Door/TriggerBlue_BP.TriggerBlue_BP_C")
    (set `self.BlueCorrect` true)
    (if (`self.OrangeCorrect`)
      (`self.SetIsOpen` true)
      (if (not (`AudioComponent.IsPlaying` _audio)) :!label _label
        (`AudioComponent.Play` _audio 0.0)))
    (else
      (set `self.BlueCorrect` false))))

(event `self.TriggerVolOrange.OnActorBeginOverlap`
  (params (OverlappedActor :type "Actor Object Reference") (OtherActor :type "Actor Object Reference"))
  (if (== (`GameplayStatics.GetObjectClass` OtherActor) "/Game/Main/Door/TriggerOrange_BP.TriggerOrange_BP_C")
    (set `self.OrangeCorrect` true)
    (if (`self.BlueCorrect`)
      (`self.SetIsOpen` true)
      (goto _label))
    (else
      (set `self.OrangeCorrect` false))))

(fn `SetIsOpen`
  (params (State :type Boolean))
  (set `self.IsOpen` State))

(fn `UserConstructionScript`)