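; Puzzle door that requires six West and East Wing trigger volumes to be overlapped by matching blue or orange trigger actors.
; Each correct overlap sets its IsCorrect flag, never cleared here, then rechecks all six.
; When all are true, it plays a rock-door sound and applies one FInterpTo step lowering the root.
; That step runs only on overlap, using the actor tick interval as delta time, because Tick is empty.
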(event `self.ReceiveTick`
  (params (DeltaSeconds :type "Float (single-precision)")))

(event `self.WestWing_TriggerVolume_Blue.OnActorBeginOverlap`
  (params (OverlappedActor :type "Actor Object Reference") (OtherActor :type "Actor Object Reference"))
  (bind _defaultsceneroot (`self.DefaultSceneRoot`))
  (bind _returnvalue (== (`GameplayStatics.GetObjectClass` OtherActor) "/Game/Main/Door/TriggerBlue_BP.TriggerBlue_BP_C"))
  (if _returnvalue
    (`KismetArrayLibrary.Array_Set` (`self.IsCorrect`) 0 _returnvalue)
    (if (`|GetArrayItem` (`self.IsCorrect`)) :!label _label
      (if (`|GetArrayItem` (`self.IsCorrect`) 1)
        (if (`|GetArrayItem` (`self.IsCorrect`) 2)
          (if (`|GetArrayItem` (`self.IsCorrect`) 3)
            (if (`|GetArrayItem` (`self.IsCorrect`) 4)
              (if (`|GetArrayItem` (`self.IsCorrect`) 5)
                (`SceneComponent.K2_SetRelativeTransform` _defaultsceneroot (`KismetMathLibrary.MakeTransform` (`KismetMathLibrary.MakeVector` 0.0 0.0 (`KismetMathLibrary.FInterpTo` (.z (.location (`SceneComponent.GetRelativeTransform` _defaultsceneroot))) -400.0 (`self.GetActorTickInterval`) 0.2))) false false)
                (`GameplayStatics.PlaySound2D` "/Game/Assets/Audio/HeavyRockDoor.HeavyRockDoor" 1.0 1.0 0.0 null null)))))))))

(event `self.WestWing_TriggerVolume_OrangeOne.OnActorBeginOverlap`
  (params (OverlappedActor :type "Actor Object Reference") (OtherActor :type "Actor Object Reference"))
  (bind _returnvalue (== (`GameplayStatics.GetObjectClass` OtherActor) "/Game/Main/Door/TriggerOrange_BP.TriggerOrange_BP_C"))
  (if _returnvalue
    (`KismetArrayLibrary.Array_Set` (`self.IsCorrect`) 1 _returnvalue)
    (goto _label)))

(event `self.WestWing_TriggerVolume_OrangeTwo.OnActorBeginOverlap`
  (params (OverlappedActor :type "Actor Object Reference") (OtherActor :type "Actor Object Reference"))
  (bind _returnvalue (== (`GameplayStatics.GetObjectClass` OtherActor) "/Game/Main/Door/TriggerOrange_BP.TriggerOrange_BP_C"))
  (if _returnvalue
    (`KismetArrayLibrary.Array_Set` (`self.IsCorrect`) 2 _returnvalue)
    (goto _label)))

(event `self.EastWing_TriggerVolume_Orange.OnActorBeginOverlap`
  (params (OverlappedActor :type "Actor Object Reference") (OtherActor :type "Actor Object Reference"))
  (bind _returnvalue (== (`GameplayStatics.GetObjectClass` OtherActor) "/Game/Main/Door/TriggerOrange_BP.TriggerOrange_BP_C"))
  (if _returnvalue
    (`KismetArrayLibrary.Array_Set` (`self.IsCorrect`) 3 _returnvalue)
    (goto _label)))

(event `self.EastWing_TriggerVolume_BlueOne.OnActorBeginOverlap`
  (params (OverlappedActor :type "Actor Object Reference") (OtherActor :type "Actor Object Reference"))
  (bind _returnvalue (== (`GameplayStatics.GetObjectClass` OtherActor) "/Game/Main/Door/TriggerBlue_BP.TriggerBlue_BP_C"))
  (if _returnvalue
    (`KismetArrayLibrary.Array_Set` (`self.IsCorrect`) 4 _returnvalue)
    (goto _label)))

(event `self.EastWing_TriggerVolume_BlueTwo.OnActorBeginOverlap`
  (params (OverlappedActor :type "Actor Object Reference") (OtherActor :type "Actor Object Reference"))
  (bind _returnvalue (== (`GameplayStatics.GetObjectClass` OtherActor) "/Game/Main/Door/TriggerBlue_BP.TriggerBlue_BP_C"))
  (if _returnvalue
    (`KismetArrayLibrary.Array_Set` (`self.IsCorrect`) 5 _returnvalue)
    (goto _label)))

(fn `UserConstructionScript`)