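; Door actor whose slab slides vertically to a target height when an actor of class Trigger_DoorOne enters its Box trigger.
; Box overlap sets IsOpen for that exact class and clears it for any other, halting movement without closing the door.
; While IsOpen, a throttled Tick eases the slab's relative Z with FInterpTo, using the tick interval as delta time.
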(event `self.ReceiveBeginPlay`
  (`self.SetActorTickInterval` 0.01))

(event `self.ReceiveTick`
  (params (DeltaSeconds :type "Float (single-precision)"))
  (bind _slabdoor_cube (`self.slabdoor_Cube`))
  (bind _target_location (`self.Target Location`))
  (bind _z (.z (.location (`SceneComponent.GetRelativeTransform` _slabdoor_cube))))
  (if (`self.IsOpen`)
    (`SceneComponent.K2_SetRelativeTransform` _slabdoor_cube (`KismetMathLibrary.MakeTransform` (`KismetMathLibrary.MakeVector` 0.0 0.0 (`KismetMathLibrary.FInterpTo` _z _target_location (`self.GetActorTickInterval`) 0.1))) false false)
    (if (not (== _z _target_location))
      (set `self.IsOpen` true))))

(event `self.Box.OnComponentBeginOverlap`
  (params (OverlappedComponent :type "PrimitiveComponent Object Reference") (OtherActor :type "Actor Object Reference") (OtherComp :type "PrimitiveComponent Object Reference") (OtherBodyIndex :type Integer) (bFromSweep :type Boolean) (SweepResult :type "HitResult Structure (by ref)"))
  ;[1 1 1] Detect Overlap
  (if (== (`GameplayStatics.GetObjectClass` OtherActor) "/Game/Main/Door/Trigger_DoorOne.Trigger_DoorOne_C")
    (set `self.IsOpen` true)
    (else
      (set `self.IsOpen` false))))

(fn `UserConstructionScript`)